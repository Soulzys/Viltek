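; BP_BoolTesting is a Geometry Script test Blueprint for procedural mesh booleans.
; On generated mesh rebuild, it appends a thin box to the target mesh and subtracts a smaller, offset, slightly taller box from it.
; The cutting box is built in a temporary compute mesh, and all compute meshes are released afterwards.
; BeginPlay, overlap and Tick are disabled stubs, and the construction script only calls its parent.
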(event EventBeginPlay
  (|CallParentFunction) ; This node is disabled and will not be called.\nDrag off pins to build functionality.
)

(event Collision|EventActorBeginOverlap
  (params (OtherActor :type Actor%20Object%20Reference))
  (|CallParentFunction OtherActor) ; This node is disabled and will not be called.\nDrag off pins to build functionality.
)

(event EventTick
  (params (DeltaSeconds :type Float%20%28single-precision%29))
  (|CallParentFunction DeltaSeconds) ; This node is disabled and will not be called.\nDrag off pins to build functionality.
)

(event Events|EventOnRebuildGeneratedMesh
  (params (TargetMesh :type Dynamic%20Mesh%20Object%20Reference))
  (bind _returnvalue (Class|GeometryScriptLibraryMeshPrimitiveFunctions|AppendBox :TargetMesh TargetMesh :DimensionZ 1e+01 :Debug 0))
  (bind _returnvalue_2 (DynamicMeshActor|AllocateComputeMesh))
  (bind _returnvalue_3 (Class|GeometryScriptLibraryMeshPrimitiveFunctions|AppendBox :TargetMesh _returnvalue_2 :Transform (Math|Transform|MakeTransform "25.000000,25.000000,0.000000" "0, 0, 0" "1.000000,1.000000,1.000000") :DimensionX 5e+01 :DimensionY 5e+01 :DimensionZ 15.0 :Debug 0))
  (GeometryScript|Booleans|ApplyMeshBoolean :TargetMesh _returnvalue :ToolMesh _returnvalue_3 :Operation "Subtract" :Debug 0)
  (DynamicMeshActor|ReleaseAllComputeMeshes))

(fn ConstructionScript
  (|CallParentFunction))