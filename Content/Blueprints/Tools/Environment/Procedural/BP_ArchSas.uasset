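; Procedural environment tool that builds a box-based mesh, named as an arch, with Geometry Script on each generated-mesh rebuild.
; It appends a base box, carves a frame-shaped cutter from two boxes on pooled compute meshes, subtracts that cutter from the base, then releases the compute meshes.
; An unconnected second boolean chain with different dimensions never runs, and the construction script only calls its parent.
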(event EventBeginPlay
  (|CallParentFunction) ; This node is disabled and will not be called.\nDrag off pins to build functionality.
)

(event Collision|EventActorBeginOverlap
  (params (OtherActor :type Actor%20Object%20Reference))
  (|CallParentFunction OtherActor) ; This node is disabled and will not be called.\nDrag off pins to build functionality.
)

(event EventTick
  (params (DeltaSeconds :type Float%20%28single-precision%29))
  (|CallParentFunction DeltaSeconds) ; This node is disabled and will not be called.\nDrag off pins to build functionality.
)

(event Events|EventOnRebuildGeneratedMesh
  (params (TargetMesh :type Dynamic%20Mesh%20Object%20Reference))
  (bind _returnvalue (Class|GeometryScriptLibraryMeshPrimitiveFunctions|AppendBox :TargetMesh TargetMesh :DimensionX 2e+02 :DimensionY 4e+01 :DimensionZ 2e+02 :Debug 0))
  (bind _returnvalue_2 (DynamicMeshActor|AllocateComputeMesh))
  (bind _returnvalue_3 (Class|GeometryScriptLibraryMeshPrimitiveFunctions|AppendBox :TargetMesh _returnvalue_2 :DimensionX 2.1e+02 :DimensionY 5e+01 :DimensionZ 2.1e+02 :Debug 0))
  (bind _returnvalue_4 (DynamicMeshActor|AllocateComputeMesh))
  (bind _returnvalue_5 (Class|GeometryScriptLibraryMeshPrimitiveFunctions|AppendBox :TargetMesh _returnvalue_4 :DimensionX 1.8e+02 :DimensionY 6e+01 :DimensionZ 1.8e+02 :Debug 0))
  (bind _returnvalue_6 (GeometryScript|Booleans|ApplyMeshBoolean :TargetMesh _returnvalue_3 :ToolMesh _returnvalue_5 :Operation "Subtract" :Debug 0))
  (GeometryScript|Booleans|ApplyMeshBoolean :TargetMesh _returnvalue :ToolMesh _returnvalue_6 :Operation "Subtract" :Debug 0)
  (DynamicMeshActor|ReleaseAllComputeMeshes))

(fn ConstructionScript
  (|CallParentFunction))