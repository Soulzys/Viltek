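; Test Blueprint for procedural mesh generation with Geometry Script, using the generated dynamic mesh rebuild event.
; On rebuild it appends an XY rectangle to the target mesh, then runs an extrude on it with zero distance.
; An unconnected triangulated-polygon node with hand-entered vertices never runs, and the construction script only calls its parent.
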(event EventBeginPlay
  (|CallParentFunction) ; This node is disabled and will not be called.\nDrag off pins to build functionality.
)

(event Collision|EventActorBeginOverlap
  (params (OtherActor :type Actor%20Object%20Reference))
  (|CallParentFunction OtherActor) ; This node is disabled and will not be called.\nDrag off pins to build functionality.
)

(event EventTick
  (params (DeltaSeconds :type Float%20%28single-precision%29))
  (|CallParentFunction DeltaSeconds) ; This node is disabled and will not be called.\nDrag off pins to build functionality.
)

(event Events|EventOnRebuildGeneratedMesh
  (params (TargetMesh :type Dynamic%20Mesh%20Object%20Reference))
  (bind _returnvalue (Class|GeometryScriptLibraryMeshPrimitiveFunctions|AppendRectangleXY :TargetMesh TargetMesh :Debug 0))
  (Class|GeometryScriptLibraryMeshModelingFunctions|ApplyMeshExtrude _returnvalue (Utilities|Struct|MakeGeometryScriptMeshExtrudeOptions 0.0 "0.000000,0.000000,1.000000" 1.0 true) 0))

(fn ConstructionScript
  (|CallParentFunction))