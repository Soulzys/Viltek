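; BP_LineTrace is a Geometry Script generated mesh actor that appears to test line tracing against procedural geometry.
; On each mesh rebuild it appends a box with no specified dimensions to the target mesh, then fires a Visibility trace between fixed points along X.
; The trace draws persistent debug and its hit result is unused; the construction script only calls its parent and the other events are disabled stubs.
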(event EventBeginPlay
  (|CallParentFunction) ; This node is disabled and will not be called.\nDrag off pins to build functionality.
)

(event Collision|EventActorBeginOverlap
  (params (OtherActor :type Actor%20Object%20Reference))
  (|CallParentFunction OtherActor) ; This node is disabled and will not be called.\nDrag off pins to build functionality.
)

(event EventTick
  (params (DeltaSeconds :type Float%20%28single-precision%29))
  (|CallParentFunction DeltaSeconds) ; This node is disabled and will not be called.\nDrag off pins to build functionality.
)

(event Events|EventOnRebuildGeneratedMesh
  (params (TargetMesh :type Dynamic%20Mesh%20Object%20Reference))
  (Utilities|FlowControl|Sequence
    (:then_0
      (Class|GeometryScriptLibraryMeshPrimitiveFunctions|AppendBox :TargetMesh TargetMesh :Debug 0))
    (:then_1
      (Collision|LineTraceByChannel "250.000000, 0,50.000000" "0.000000, 0,50.000000" "TraceTypeQuery1" false 0 "Persistent" true "(R=1.000000,G=0.000000,B=0.000000,A=1.000000)" "(R=0.000000,G=1.000000,B=0.000000,A=1.000000)" 25.0))))

(fn ConstructionScript
  (|CallParentFunction))