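; Procedural wall tool, a Geometry Script generated-mesh actor that builds a box wall from width, thickness and height parameters on rebuild.
; With ExtendWall on, it adds a 90-degree revolved bend at the top and a rotated box that continues the wall past the curve.
; Both pieces are built in temporary compute meshes and boolean-unioned into the wall, after which the compute meshes are released and split normals are recomputed.
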(event EventBeginPlay
  (|CallParentFunction) ; This node is disabled and will not be called.\nDrag off pins to build functionality.
)

(event Collision|EventActorBeginOverlap
  (params (OtherActor :type Actor%20Object%20Reference))
  (|CallParentFunction OtherActor) ; This node is disabled and will not be called.\nDrag off pins to build functionality.
)

(event EventTick
  (params (DeltaSeconds :type Float%20%28single-precision%29))
  (|CallParentFunction DeltaSeconds) ; This node is disabled and will not be called.\nDrag off pins to build functionality.
)

(event Events|EventOnRebuildGeneratedMesh
  (params (TargetMesh :type Dynamic%20Mesh%20Object%20Reference))
  (bind _wallthickness (Variables|Default|GetWallThickness))
  (bind _wallwidth (Variables|Default|GetWallWidth))
  (bind _output_get (Variables|Default|SetDynamicMesh TargetMesh))
  (Class|GeometryScriptLibraryMeshPrimitiveFunctions|AppendBox :TargetMesh _output_get :DimensionX (Variables|Default|GetWallWidth) :DimensionY (Variables|Default|GetWallThickness) :DimensionZ (Variables|Default|GetWallHeight) :Debug 0)
  (if (Variables|Default|GetExtendWall)
    (bind _returnvalue (DynamicMeshActor|AllocateComputeMesh))
    (bind _returnvalue_2 (Class|GeometryScriptLibraryMeshPrimitiveFunctions|AppendRevolvePolygon :TargetMesh _returnvalue :Transform (Math|Transform|MakeTransform (Math|Vector|MakeVector (/ _wallwidth 2.0) (+ (Variables|Default|GetRadius) (/ _wallthickness 2.0)) (Variables|Default|GetWallHeight)) "0,90.000000,90.000000" "1.000000,1.000000,1.000000") :PolygonVertices (Utilities|Array|MakeArray (Math|Vector2D|MakeVector2D 0.0 0.0) (Math|Vector2D|MakeVector2D _wallthickness 0.0) (Math|Vector2D|MakeVector2D _wallthickness _wallwidth) (Math|Vector2D|MakeVector2D 0.0 _wallwidth)) :RevolveOptions (Utilities|Struct|MakeGeometryScriptRevolveOptions 9e+01 -1.8e+02 false false 3e+01 false true) :Radius (Variables|Default|GetRadius) :Debug 0))
    (bind _returnvalue_3 (GeometryScript|Booleans|ApplyMeshBoolean :TargetMesh (Variables|Default|GetDynamicMesh) :ToolMesh _returnvalue_2 :Operation "Union" :Debug 0))
    (bind _returnvalue_4 (DynamicMeshActor|AllocateComputeMesh))
    (bind _returnvalue_5 (Class|GeometryScriptLibraryMeshPrimitiveFunctions|AppendBox :TargetMesh _returnvalue_4 :DimensionX (Variables|Default|GetWallWidth) :DimensionY (Variables|Default|GetWallThickness) :DimensionZ (Variables|Default|GetExtendedLength) :Debug 0))
    (bind _returnvalue_6 (GeometryScript|Booleans|ApplyMeshBoolean :TargetMesh _returnvalue_3 :ToolMesh _returnvalue_5 :ToolTransform (Math|Transform|MakeTransform (Math|Vector|MakeVector 0.0 (+ (/ (Variables|Default|GetWallThickness) 2.0) (Variables|Default|GetRadius)) (+ (+ (/ (Variables|Default|GetWallThickness) 2.0) (Variables|Default|GetWallHeight)) (Variables|Default|GetRadius))) "0, 0,90.000000" "1.000000,1.000000,1.000000") :Operation "Union" :Debug 0))
    (Variables|Default|SetDynamicMesh _returnvalue_6)
    (DynamicMeshActor|ReleaseAllComputeMeshes)
    (bind _returnvalue_7 (Class|GeometryScriptLibraryMeshNormalsFunctions|ComputeSplitNormals :TargetMesh (Variables|Default|GetDynamicMesh) :Debug 0))
    (Variables|Default|SetDynamicMesh _returnvalue_7)))

(fn ConstructionScript
  (|CallParentFunction))