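; BP_BaseDynamicWall is a procedural environment tool that generates a box wall with a cutout using Geometry Script.
; On mesh rebuild it extrudes a plain or rounded rectangle into a cutter and boolean-subtracts it from the wall at a configurable location.
; The cutter gets its own material ID, so the cut faces take a separate material.
; Optional angle-based polygroup bevels and split normals precede UV recomputation and scaling.
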(event EventBeginPlay)

(event Collision|EventActorBeginOverlap
  (params (OtherActor :type Actor%20Object%20Reference)))

(event EventTick
  (params (DeltaSeconds :type Float%20%28single-precision%29)))

(event Events|EventOnRebuildGeneratedMesh
  (params (TargetMesh :type Dynamic%20Mesh%20Object%20Reference))
  (bind _wallsize (Variables|Default|GetWallSize))
  (bind _cutoutsize (Variables|Default|GetCutoutSize))
  (bind _cutoutsize_2 (Variables|Default|GetCutoutSize))
  (Variables|Default|SetDynamicMesh TargetMesh)
  (Utilities|FlowControl|Sequence
    (:then_0
      ;[1 1 1] CREATE WALL
      (Class|GeometryScriptLibraryMeshPrimitiveFunctions|AppendBox :TargetMesh (Variables|Default|GetDynamicMesh) :DimensionX (.x _wallsize) :DimensionY (.y _wallsize) :DimensionZ (.z _wallsize) :Debug 0))
    (:then_1
      (if (Variables|Default|GetbIsCutoutRounded)
        ;[1 1 1] CREATE ROUNDED CUTOUT
        (bind _returnvalue (DynamicMeshActor|AllocateComputeMesh))
        (bind _returnvalue_2 (Class|GeometryScriptLibraryMeshPrimitiveFunctions|AppendRoundRectangleXY :TargetMesh _returnvalue :Transform (Math|Transform|MakeTransform "0, 0, 0" "0, 0,90.000000" "1.000000,1.000000,1.000000") :DimensionX (.x _cutoutsize_2) :DimensionY (.z _cutoutsize_2) :CornerRadius (Variables|Default|GetCorner%20Radius) :StepsRound (Variables|Default|GetSteps%20Round) :Debug 0))
        (Variables|Default|SetCutoutMesh _returnvalue_2)
        (else
          ;[1 1 1] CREATE CUTOUT
          (bind _returnvalue_3 (DynamicMeshActor|AllocateComputeMesh))
          (bind _returnvalue_4 (Class|GeometryScriptLibraryMeshPrimitiveFunctions|AppendRectangleXY :TargetMesh _returnvalue_3 :Transform (Math|Transform|MakeTransform "0, 0, 0" "0, 0,90.000000" "1.000000,1.000000,1.000000") :DimensionX (.x _cutoutsize) :DimensionY (.z _cutoutsize) :Debug 0))
          (Variables|Default|SetCutoutMesh _returnvalue_4))))
    (:then_2
      ;[1 1 1] EXTRUDE CUTOUT
      (bind _returnvalue_5 (Class|GeometryScriptLibraryMeshModelingFunctions|ApplyMeshExtrude (Variables|Default|GetCutoutMesh) (Utilities|Struct|MakeGeometryScriptMeshExtrudeOptions (.y (Variables|Default|GetCutoutSize)) "0.000000,1.000000,0.000000" 1.0 true) 0))
      (GeometryScript|Materials|RemapMaterialIDs _returnvalue_5 0 1 0)
      (Variables|Default|SetCutoutMesh _returnvalue_5))
    (:then_3
      ;[1 1 1] APPLY CUTOUT BOOLEAN
      (bind _returnvalue_6 (GeometryScript|Booleans|ApplyMeshBoolean :TargetMesh (Variables|Default|GetDynamicMesh) :ToolMesh (Variables|Default|GetCutoutMesh) :ToolTransform (Math|Transform|MakeTransform (Variables|Default|GetCutoutLocation) "0, 0, 0" "1.000000,1.000000,1.000000") :Operation "Subtract" :Debug 0))
      (Variables|Default|SetDynamicMesh _returnvalue_6))
    (:then_4
      ;[1 1 1] DO BEVELS
      (if (Variables|Default|GetbIsBeveled)
        (bind _returnvalue_7 (Class|GeometryScriptLibraryMeshPolygroupFunctions|ComputePolygroupsfromAngleThreshold :TargetMesh (Variables|Default|GetDynamicMesh) :CreaseAngle 25.0 :Debug 0))
        (bind _returnvalue_8 (Class|GeometryScriptLibraryMeshModelingFunctions|ApplyMeshPolygroupBevel _returnvalue_7 (Utilities|Struct|MakeGeometryScriptMeshBevelOptions (Variables|Default|GetBevelAmount) false 0 false "(Min=(X=0.000000,Y=0.000000,Z=0.000000),Max=(X=0.000000,Y=0.000000,Z=0.000000),IsValid=0)" "0.000000,0.000000,0.000000|0.000000,0.000000,-0.000000|1.000000,1.000000,1.000000" true) 0))
        (bind _returnvalue_9 (Class|GeometryScriptLibraryMeshNormalsFunctions|ComputeSplitNormals :TargetMesh _returnvalue_8 :SplitOptions (Utilities|Struct|MakeGeometryScriptSplitNormalsOptions true 25.0 false "(bDefaultLayer=True,ExtendedLayerIndex=0)") :Debug 0))
        (Variables|Default|SetDynamicMesh _returnvalue_9)))
    (:then_5
      ;[1 1 1] SETUP MATERIALS
      (Class|DynamicMeshComponent|ConfigureMaterialSet (Variables|Default|GetDynamicMeshComponent) (Utilities|Array|MakeArray (Variables|Default|GetWallMaterial) (Variables|Default|GetCutoutMaterial))))
    (:then_6
      ;[1 1 1] RECOMPUTE AND SCALE UVS
      (bind _returnvalue_10 (Class|GeometryScriptLibraryMeshUVFunctions|RecomputeMeshUVs :TargetMesh (Variables|Default|GetDynamicMesh) :Debug 0))
      (GeometryScript|UVs|ScaleMeshUVs :TargetMesh _returnvalue_10 :Scale (Math|Vector2D|MakeVector2D (Variables|Default|GetUV_ScaleX) (Variables|Default|GetUV_ScaleY)) :Debug 0))))

(fn ConstructionScript
  (|CallParentFunction))